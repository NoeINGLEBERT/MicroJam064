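; BP_Goblins is a goblin trap hazard that, once activated through DoStuff, fights any dwarf entering its sphere.
; DoStuff plays goblin sounds and applies a material and outline to three trap-floor meshes.
; The dwarf's weapon and fog state decide each fight: sure death, coin flip or sure win, with Sword faring best.
; A losing dwarf is destroyed with blood and sound, while losing goblins spawn a fresh BP_Goblins before destroying themselves.
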(event `self.DoStuff`
  (bind _sm_prop_trap_floor_dungeon_05 (`self.SM_PROP_trap_floor_dungeon_05`))
  (set `self.Active` true)
  (`GameplayStatics.PlaySoundAtLocation` "/Game/Song/SC_GoblinsFight.SC_GoblinsFight" (`SceneComponent.K2_GetComponentLocation` (`self.Sphere`)) (struct) 1.0 1.0 0.0 "/Game/Song/SA_Dwarf.SA_Dwarf" null null null)
  (`PrimitiveComponent.SetMaterial` _sm_prop_trap_floor_dungeon_05 0 "/Game/Goblins/NewMaterial.NewMaterial")
  (`PrimitiveComponent.SetMaterial` (`self.SM_PROP_trap_floor_dungeon_06`) 0 "/Game/Goblins/NewMaterial.NewMaterial")
  (`PrimitiveComponent.SetMaterial` (`self.SM_PROP_trap_floor_dungeon_07`) 0 "/Game/Goblins/NewMaterial.NewMaterial")
  (`MeshComponent.SetOverlayMaterial` _sm_prop_trap_floor_dungeon_05 "/Game/Materials/Outline.Outline")
  (`MeshComponent.SetOverlayMaterial` (`self.SM_PROP_trap_floor_dungeon_07`) "/Game/Materials/Outline.Outline")
  (`MeshComponent.SetOverlayMaterial` (`self.SM_PROP_trap_floor_dungeon_06`) "/Game/Materials/Outline.Outline"))

(event `self.Sphere.OnComponentBeginOverlap`
  (params (OverlappedComponent :type "PrimitiveComponent Object Reference") (OtherActor :type "Actor Object Reference") (OtherComp :type "PrimitiveComponent Object Reference") (OtherBodyIndex :type Integer) (bFromSweep :type Boolean) (SweepResult :type "HitResult Structure (by ref)"))
  (bind _returnvalue (`SceneComponent.K2_GetComponentLocation` (`self.Sphere`)))
  (if (`self.Active`)
    (bind _asbp_dwarf (cast `/Game/Blueprints/BP_Dwarf` OtherActor))
    (`GameplayStatics.PlaySoundAtLocation` "/Game/Song/SC-DwarfFight.SC-DwarfFight" _returnvalue (struct) 1.0 1.0 0.0 "/Game/Song/SA_Dwarf.SA_Dwarf" null null null)
    (`GameplayStatics.PlaySoundAtLocation` "/Game/Song/SC_GoblinsFight.SC_GoblinsFight" _returnvalue (struct) 1.0 1.0 0.0 "/Game/Song/SA_Dwarf.SA_Dwarf" null null null)
    (`GameplayStatics.PlaySoundAtLocation` "/Game/Song/dragon-studio-sword-fight-393849.dragon-studio-sword-fight-393849" (0.0 0.0 0.0) (struct) 1.0 1.0 0.0 "/Game/Song/SA_Dwarf.SA_Dwarf" null null null)
    (switch `/Game/Data/EWeapon` (`/Game/Blueprints/BP_Dwarf.Weapon` _asbp_dwarf)
      (:`NewEnumerator0`
        (bind _isinfog (`/Game/Blueprints/BP_Dwarf.IsInFog` _asbp_dwarf))
        (if _isinfog :!label _label
          (`NiagaraFunctionLibrary.SpawnSystemAtLocation` "/Game/Niaga/RedBlood.RedBlood" (`self.K2_GetActorLocation` _asbp_dwarf) :!label _label_2)
          (`GameplayStatics.PlaySoundAtLocation` "/Game/Song/SC_DwarfDeath.SC_DwarfDeath" (`SceneComponent.K2_GetComponentLocation` (`self.Sphere`)) (struct) 1.0 1.0 0.0 "/Game/Song/SA_Dwarf.SA_Dwarf" null null null)
          (`self.K2_DestroyActor` _asbp_dwarf)
          (else
            (if (`KismetMathLibrary.RandomBool`) :!label _label_3
              (goto _label_2)
              (else
                (`|SpawnActorFromClass` "BP_Goblins_C" (`self.GetTransform`) "Undefined" "MultiplyWithRoot" null null :!label _label_4)
                (for _array_element (`|MakeArray` (`self.SM_PROP_trap_floor_dungeon_06`) (`self.SM_PROP_trap_floor_dungeon_07`) (`self.SM_PROP_trap_floor_dungeon_05`))
                  (`NiagaraFunctionLibrary.SpawnSystemAtLocation` "/Game/Niaga/GreenBlood.GreenBlood" (+ (`SceneComponent.K2_GetComponentLocation` _array_element) (0.0 0.0 50.0))))
                (`GameplayStatics.PlaySoundAtLocation` "/Game/Song/SC_GloblinsDeath.SC_GloblinsDeath" (`SceneComponent.K2_GetComponentLocation` (`self.Sphere`)) (struct) 1.0 1.0 0.0 "/Game/Song/SA_Dwarf.SA_Dwarf" null null null)
                (`self.K2_DestroyActor`))))))
      (:`NewEnumerator1`
        (if _isinfog
          (goto _label_3)
          (else
            (goto _label_4))))
      (:`NewEnumerator2`
        (goto _label)))))

(fn `UserConstructionScript`)