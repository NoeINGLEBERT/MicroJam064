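; Player Blueprint for a game of hindering treasure-seeking dwarves, handling mouse interaction, scroll movement and the HUD.
; Scroll input moves the actor diagonally within clamped limits.
; Left-click traces under the cursor to show dwarf trait popups, offer paid bridge demolition or spike building, or harvest mana from treasure.
; Right-click sends the fog to the traced point if mana allows, draining the cost gradually through a DoN-and-Delay loop.
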(event `self.ReceiveBeginPlay`
  (`EnhancedInputSubsystemInterface.AddMappingContext` (pcsubsystem `EnhancedInputLocalPlayerSubsystem` (`GameplayStatics.GetPlayerController` 0)) "/Game/Inputs/IMC_Game.IMC_Game" 0 (struct))
  (bind _returnvalue (`|CreateWidget` "/Game/Widgets/WBP_HUD.WBP_HUD_C"))
  (bind _output_get (set `self.HUD` _returnvalue))
  (`UserWidget.AddToViewport` _output_get 0))

(event `EnhancedInput|/Game/Inputs/IA_Scroll`
  (params (ActionValue :type "Float (double-precision)") (ElapsedSeconds :type "Float (double-precision)") (TriggeredSeconds :type "Float (double-precision)") (InputAction :type "InputAction Object Reference" :default "/Game/Inputs/IA_Scroll.IA_Scroll"))
  (bind _returnvalue (+ ActionValue (`self.Scroll`)))
  (:`Triggered`
    (if (and (> _returnvalue -40.0) (< _returnvalue 2.0))
      (set `self.Scroll` _returnvalue)
      (`self.K2_SetActorLocation` (+ (`self.K2_GetActorLocation`) (* ActionValue (3.0 3.0 3.0) 30.0))))))

(event `Key|LeftMouseButton`
  (params (Key :type "Key Structure"))
  (bind _hud (`self.HUD`))
  (bind _hud_2 (`self.HUD`))
  (bind (_worldlocation _worlddirection) (`PlayerController.DeprojectMousePositionToWorld` (`GameplayStatics.GetPlayerController` 0)))
  (:`Pressed`
    (`/Game/Widgets/WBP_HUD.TogglePop` _hud false)
    (bind (_outhit _returnvalue) (`KismetSystemLibrary.LineTraceSingle` _worldlocation (+ _worldlocation (* _worlddirection 10000.0)) "TraceTypeQuery1"))
    (if _returnvalue
      (bind (_bblockinghit _binitialoverlap _time _distance _location _impactpoint _normal _impactnormal _physmat _hitactor) (`GameplayStatics.BreakHitResult` _outhit))
      (bind _asbp_dwarf (cast `/Game/Blueprints/BP_Dwarf` _hitactor)
        (:`then`
          (`/Game/Widgets/WBP_HUD.TogglePop` _hud true)
          (bind _clothes (`/Game/Blueprints/BP_Dwarf.Clothes` _asbp_dwarf))
          (bind _hair (`/Game/Blueprints/BP_Dwarf.Hair` _asbp_dwarf))
          (bind _weapon (`/Game/Blueprints/BP_Dwarf.Weapon` _asbp_dwarf))
          (`/Game/Widgets/WBP_HUD.UpdatePopUp` _hud (`/Game/Blueprints/BP_Dwarf.Name` _asbp_dwarf) (`|FormatText` "{Clothes} {Hair}... with a {Weapon}!" (`|GetEnumeratorNameAsString` _clothes) (`|GetEnumeratorNameAsString` _hair) (`|GetEnumeratorNameAsString` _weapon)) (`|FormatText` "{Clothes} \n \n{Hair} \n \n{Weapon}" (select `/Game/Data/EClothes` _clothes :`NewEnumerator0` "- Wannabe king, wants the Heart of the Mountain and nothing else" :`NewEnumerator1` "- Completely broke, will settle for the first treasure he finds" :`NewEnumerator2` "- The Goblins took the mountain from the Ice Dwarves and they aren't known to forget grudges, this one isn't here for the gold..." :!type "Text") (select `/Game/Data/EHair` _hair :`NewEnumerator0` "- Flee when in the fog, but will muster the courage to go again " :`NewEnumerator1` "- Unbelievably stubborn, moves straight trough the fog" :`NewEnumerator2` "- Not the shiniest gem of the mine, moves randomly in the fog" :!type "Text") (select `/Game/Data/EWeapon` _weapon :`NewEnumerator0` "- A mastercraftsman, with a hammer and a few planks, any chasm can be crossed" :`NewEnumerator1` "- Has a sword, usefull for cutting down the nasty green-skins" :`NewEnumerator2` "- Steady as a rock, it will take more than a few spikes to get rid of him" :!type "Text"))))
        (:`CastFailed`
          (bind _asbp_bridge (cast `/Game/Blueprints/BP_Bridge` _hitactor)
            (:`then`
              (`/Game/Widgets/WBP_HUD.TogglePop` _hud true)
              (`/Game/Widgets/WBP_HUD.UpdatePopUp` _hud "Bridge" "Hazardous crossing" "Rickety bridge easily demolished. \n \nFalling off a bridge is a privielege usually reserved to giant flame demons of pure darkness, but it might work on dwarves as well if you give it a shot.")
              (`/Game/Widgets/WBP_HUD.ShowButton` _hud true 50 "CLICK HERE TO DESTROY" _asbp_bridge))
            (:`CastFailed`
              (bind _asbp_spike (cast `/Game/Blueprints/BP_Spike` _hitactor)
                (:`then`
                  (`/Game/Widgets/WBP_HUD.TogglePop` _hud true)
                  (`/Game/Widgets/WBP_HUD.UpdatePopUp` _hud "Spikes" "Carefull where you step!" "You can help the goblins out by building spike traps. \n \nThey aren't on the path though, you'll have to trick dwarves into stepping on them. \n \nGoblin traps aren't sturdy, once it kills a dwarf, it will break apart.")
                  (`/Game/Widgets/WBP_HUD.ShowButton` _hud true 20 "CLICK HERE TO BUILD" _asbp_spike))
                (:`CastFailed`
                  (bind _asbp_treasure (cast `/Game/Blueprints/BP_Treasure` _hitactor))
                  (set `/Game/Widgets/WBP_HUD.mANA` (+ (`/Game/Widgets/WBP_HUD.mANA` _hud_2) (`/Game/Blueprints/BP_Treasure.mANAPERCLICK` _asbp_treasure)) _hud_2)))))))
      (else
        (`/Game/Widgets/WBP_HUD.TogglePop` _hud false)))))

(event `Key|RightMouseButton`
  (params (Key :type "Key Structure"))
  (bind _hud (`self.HUD`))
  (bind (_worldlocation _worlddirection) (`PlayerController.DeprojectMousePositionToWorld` (`GameplayStatics.GetPlayerController` 0)))
  (bind _mana (`/Game/Widgets/WBP_HUD.mANA` _hud))
  (:`Pressed`
    (`/Game/Widgets/WBP_HUD.TogglePop` (`self.HUD`) false)
    (bind (_outhit _returnvalue) (`KismetSystemLibrary.LineTraceSingle` _worldlocation (+ _worldlocation (* _worlddirection 10000.0)) "TraceTypeQuery1"))
    (if _returnvalue
      (if (>= _mana 10)
        (`UserWidget.PlayAnimationForward` _hud (`/Game/Widgets/WBP_HUD.CONSUME` _hud) 1.0 false)
        (bind _returnvalue_2 (`GameplayStatics.GetActorOfClass` "/Game/Blueprints/BP_Fog.BP_Fog_C"))
        (set `/Game/Blueprints/BP_Fog.TargetPosition` (`.Location` (`GameplayStatics.BreakHitResult` _outhit)) _returnvalue_2)
        (`|ExecutionSequence`
          (:`then_0`
            (goto _label :!via `Reset`))
          (:`then_1`
            (`/Engine/EditorBlueprintResources/StandardMacros.Do N` 10 :!label _label
              (:`Exit`
                (set `/Game/Widgets/WBP_HUD.mANA` (`KismetMathLibrary.Max` (+ _mana -1)) _hud)
                (`KismetSystemLibrary.Delay` 0.05)
                (goto _label)))))
        (else
          (`UserWidget.PlayAnimationForward` _hud (`/Game/Widgets/WBP_HUD.NotEnoughMana` _hud) 1.0 false))))))

(event `Key|LeftMouseButton`
  (params (Key :type "Key Structure")))

(fn `UserConstructionScript`)