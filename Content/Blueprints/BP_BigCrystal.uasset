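; BP_BigCrystal is a large crystal actor that shatters when the dwarf touches it, apparently as the game's ending.
; A capsule overlap with BP_Dwarf fires once, enables physics on four crystal mesh parts and plays an ice impact sound.
; Each part gets a radial impulse from the actor's location to blow it apart, and after a short delay "THE END" is printed.
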(event `self.Capsule.OnComponentBeginOverlap`
  (params (OverlappedComponent :type "PrimitiveComponent Object Reference") (OtherActor :type "Actor Object Reference") (OtherComp :type "PrimitiveComponent Object Reference") (OtherBodyIndex :type Integer) (bFromSweep :type Boolean) (SweepResult :type "HitResult Structure (by ref)"))
  (bind _gc_crystal_l3 (`self.GC_Crystal_L3`))
  (cast `/Game/Blueprints/BP_Dwarf` OtherActor)
  (`/Engine/EditorBlueprintResources/StandardMacros.DoOnce` false
    (:`Completed`
      (`PrimitiveComponent.SetSimulatePhysics` _gc_crystal_l3 true)
      (`PrimitiveComponent.SetSimulatePhysics` (`self.GC_Crystal_L2`) true)
      (`PrimitiveComponent.SetSimulatePhysics` (`self.GC_Crystal_L1`) true)
      (`PrimitiveComponent.SetSimulatePhysics` (`self.GC_Crystal_L`) true)
      (`GameplayStatics.PlaySound2D` "/Game/Song/dragon-studio-ice-spell-impact-448563.dragon-studio-ice-spell-impact-448563" 1.0 1.0 0.0 null null)
      (for _array_element (`|MakeArray` _gc_crystal_l3 (`self.GC_Crystal_L2`) (`self.GC_Crystal_L1`) (`self.GC_Crystal_L`))
        (`PrimitiveComponent.AddRadialImpulse` _array_element (`self.K2_GetActorLocation`) 500.0 10000.0 "RIF_Constant" false))
      (`KismetSystemLibrary.Delay` 3.0)
      (`KismetSystemLibrary.PrintString` "THE END"))))

(fn `UserConstructionScript`)