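; BP_Spike is a spike floor trap that kills BP_Dwarf actors touching its sphere while it is active.
; The DoStuff event arms it by setting Active and changing materials and outline overlays on both meshes.
; On a kill it plays a Niagara effect at the dwarf and destroys it.
; The trap then resets by spawning a fresh BP_Spike at its own transform and destroying itself.
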(event `/Game/Blueprints/BPI_DoStuff.DoStuff`
  (bind _staticmesh (`self.StaticMesh`))
  (bind _sm_prop_trap_floor_dungeon_05 (`self.SM_PROP_trap_floor_dungeon_05`))
  (set `self.Active` true)
  (`PrimitiveComponent.SetMaterial` _staticmesh 0 "/Game/Fantastic_Dungeon_Pack/materials/MI_metal_dungeon_03.MI_metal_dungeon_03")
  (`MeshComponent.SetOverlayMaterial` _staticmesh "/Game/Materials/OutlineSpike.OutlineSpike")
  (`PrimitiveComponent.SetMaterial` _sm_prop_trap_floor_dungeon_05 0 "/Game/Fantastic_Dungeon_Pack/materials/MI_metal_dungeon_01.MI_metal_dungeon_01")
  (`MeshComponent.SetOverlayMaterial` _sm_prop_trap_floor_dungeon_05 "/Game/Materials/Outline.Outline"))

(event `self.Sphere.OnComponentBeginOverlap`
  (params (OverlappedComponent :type "PrimitiveComponent Object Reference") (OtherActor :type "Actor Object Reference") (OtherComp :type "PrimitiveComponent Object Reference") (OtherBodyIndex :type Integer) (bFromSweep :type Boolean) (SweepResult :type "HitResult Structure (by ref)"))
  (bind _asbp_dwarf (cast `/Game/Blueprints/BP_Dwarf` OtherActor))
  (if (`self.Active`)
    (`NiagaraFunctionLibrary.SpawnSystemAtLocation` "/Game/Niaga/NewNiagaraSystem.NewNiagaraSystem" (`self.K2_GetActorLocation` _asbp_dwarf))
    (`self.K2_DestroyActor` _asbp_dwarf)
    (`|SpawnActorFromClass` "BP_Spike_C" (`self.GetTransform`) "Undefined" "MultiplyWithRoot" null null)
    (`self.K2_DestroyActor`)))

(fn `UserConstructionScript`)