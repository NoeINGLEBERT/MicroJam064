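; Dwarf AI character that walks to BP_BigCrystal, with random hair, clothes, weapon and data-table name rolled on spawn.
; A ping-pong timeline lerps body part transforms for running, and Tick swaps between that moving mesh set and an idle set by speed.
; Inside BP_Fog, navigation stops and hair type drives velocity: Coward backward, Elder forward, Fool toward periodically rerolled random directions.
; Reaching the crystal sets Cliff, briefly forcing forward velocity.
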(event `self.ReceiveBeginPlay`
  (`|ExecutionSequence`
    (:`then_0`
      (`self.Init`)
      (`TimelineComponent.SetPlayRate` (`self.Timeline`) 2.0)
      (bind (_direction _alpha) (`Timeline|Timeline` :!label _label)
        (:`Update`
          (`SceneComponent.K2_SetRelativeTransform` (`self.Body`) (`KismetMathLibrary.TLerp` (`self.BodyTransform_RunA`) (`self.BodyTransform_RunB`) _alpha) false false)
          (`SceneComponent.K2_SetRelativeTransform` (`self.Head`) (`KismetMathLibrary.TLerp` (`self.HeadTransform_RunA`) (`self.HeadTransform_RunB`) _alpha) false false)
          (`SceneComponent.K2_SetRelativeTransform` (`self.RightFoot`) (`KismetMathLibrary.TLerp` (`self.RightFootTransform_RunA`) (`self.RightFootTransform_RunB`) _alpha) false false)
          (`SceneComponent.K2_SetRelativeTransform` (`self.LeftFoot`) (`KismetMathLibrary.TLerp` (`self.LeftFootTransform_RunA`) (`self.LeftFootTransform_RunB`) _alpha) false false))
        (:`Finished`
          (switch `ETimelineDirection` _direction
            (:`Forward`
              (goto _label :!via `Reverse`))
            (:`Backward`
              (goto _label))))))
    (:`then_1`
      (set `self.RandomDir` (`KismetMathLibrary.RandomUnitVectorInConeInDegrees` (`self.GetActorForwardVector`) 60.0) :!label _label_2)
      (`KismetSystemLibrary.Delay` (`KismetMathLibrary.RandomFloatInRange` 0.5 1.0))
      (goto _label_2))))

(event `self.ReceiveTick`
  (params (DeltaSeconds :type "Float (single-precision)"))
  (bind _returnvalue (`self.GetActorForwardVector`))
  (bind _charactermovement (`self.CharacterMovement`))
  (bind _returnvalue_2 (* _returnvalue 300.0))
  (bind (_velocity_x _velocity_y _velocity_z) (`KismetMathLibrary.BreakVector` (`MovementComponent.Velocity` _charactermovement)))
  (bind _returnvalue_3 (> (`KismetMathLibrary.VSize` (`MovementComponent.Velocity` (`self.CharacterMovement`))) 10.0))
  (`SceneComponent.SetVisibility` (`self.Body1`) (not _returnvalue_3) false)
  (`SceneComponent.SetVisibility` (`self.RightFoot1`) (not _returnvalue_3) false)
  (`SceneComponent.SetVisibility` (`self.LeftFoot1`) (not _returnvalue_3) false)
  (`SceneComponent.SetVisibility` (`self.Head1`) (not _returnvalue_3) false)
  (`SceneComponent.SetVisibility` (`self.Hand1`) (not _returnvalue_3) false)
  (`SceneComponent.SetVisibility` (`self.WeaponMesh1`) (not _returnvalue_3) false)
  (`SceneComponent.SetVisibility` (`self.Body`) _returnvalue_3 false)
  (`SceneComponent.SetVisibility` (`self.Hand`) _returnvalue_3 false)
  (`SceneComponent.SetVisibility` (`self.LeftFoot`) _returnvalue_3 false)
  (`SceneComponent.SetVisibility` (`self.RightFoot`) _returnvalue_3 false)
  (`SceneComponent.SetVisibility` (`self.Head`) _returnvalue_3 false)
  (`SceneComponent.SetVisibility` (`self.WeaponMesh`) _returnvalue_3 false)
  (if (`self.IsInFog`)
    (set `MovementComponent.Velocity` (`KismetMathLibrary.MakeVector` (.x (select `/Game/Data/EHair` (`self.Hair`) :`NewEnumerator0` (* _returnvalue -300.0) :`NewEnumerator1` _returnvalue_2 :`NewEnumerator2` (* (`KismetMathLibrary.VInterpTo_Constant` _returnvalue (`self.RandomDir`) DeltaSeconds 1000.0) 300.0))) (.y (select `/Game/Data/EHair` (`self.Hair`) :`NewEnumerator0` (* _returnvalue -300.0) :`NewEnumerator1` _returnvalue_2 :`NewEnumerator2` (* (`KismetMathLibrary.VInterpTo_Constant` _returnvalue (`self.RandomDir`) DeltaSeconds 1000.0) 300.0))) _velocity_z) _charactermovement)
    (elif (`self.Cliff`)
      (if (`self.Cliff`) :!label _label_3
        (set `MovementComponent.Velocity` (`KismetMathLibrary.MakeVector` (.x _returnvalue_2) (.y _returnvalue_2) _velocity_z) _charactermovement)
        (`KismetSystemLibrary.Delay` 0.5)
        (set `self.Cliff` false))
      (else
        (bind _returnvalue_4 (`GameplayStatics.GetActorOfClass` "/Game/Blueprints/BP_BigCrystal.BP_BigCrystal_C"))
        (if (not (> (`KismetMathLibrary.VSize` (`MovementComponent.Velocity` (`self.CharacterMovement`))) 10.0))
          (set `self.Cliff` false)
          (`|AIMoveTo` self (`self.K2_GetActorLocation` _returnvalue_4) null
            (:`OnSuccess`
              (set `self.Cliff` true)
              (goto _label_3))
            (:`OnFail`
              (goto _label_3))))))))

(event `self.CapsuleComponent.OnComponentBeginOverlap`
  (params (OverlappedComponent :type "PrimitiveComponent Object Reference") (OtherActor :type "Actor Object Reference") (OtherComp :type "PrimitiveComponent Object Reference") (OtherBodyIndex :type Integer) (bFromSweep :type Boolean) (SweepResult :type "HitResult Structure (by ref)"))
  (cast `/Game/Blueprints/BP_Fog` OtherActor)
  (`Controller.StopMovement` (`AIBlueprintHelperLibrary.GetAIController` self))
  (set `self.IsInFog` true))

(event `self.CapsuleComponent.OnComponentEndOverlap`
  (params (OverlappedComponent :type "PrimitiveComponent Object Reference") (OtherActor :type "Actor Object Reference") (OtherComp :type "PrimitiveComponent Object Reference") (OtherBodyIndex :type Integer))
  (cast `/Game/Blueprints/BP_Fog` OtherActor)
  (set `self.IsInFog` false))

(fn `Init`
  (bind _weaponmesh1 (`self.WeaponMesh1`))
  (bind _weapon (`self.Weapon`))
  (bind _returnvalue (select `/Game/Data/EWeapon` _weapon :`NewEnumerator0` "/Game/Dwarf/Meshes/SM_DwarfHammer.SM_DwarfHammer" :`NewEnumerator1` "/Game/Fantastic_Dungeon_Pack/meshes/props/tools/SM_PROP_weapon_sword_dungeon_02.SM_PROP_weapon_sword_dungeon_02" :`NewEnumerator2` "/Game/Fantastic_Dungeon_Pack/meshes/props/tools/SM_PROP_weapon_shield_dungeon_02.SM_PROP_weapon_shield_dungeon_02" :!type "StaticMesh Object Reference"))
  (set `self.Hair` (`KismetArrayLibrary.Array_Random` (`|MakeArray` "NewEnumerator0" "NewEnumerator1" "NewEnumerator2" :!type "/Game/Data/EHair Enum")))
  (set `self.Clothes` (`KismetArrayLibrary.Array_Random` (`|MakeArray` "NewEnumerator0" "NewEnumerator1" "NewEnumerator2" :!type "/Game/Data/EClothes Enum")))
  (set `self.Weapon` (`KismetArrayLibrary.Array_Random` (`|MakeArray` "NewEnumerator0" "NewEnumerator1" "NewEnumerator2" :!type "/Game/Data/EWeapon Enum")))
  (`PrimitiveComponent.SetMaterial` (`self.Head1`) 0 (select `/Game/Data/EHair` (`self.Hair`) :`NewEnumerator0` "/Game/Dwarf/Hair/MI_BlondHair.MI_BlondHair" :`NewEnumerator1` "/Game/Dwarf/Hair/MI_GreyHair.MI_GreyHair" :`NewEnumerator2` "/Game/Dwarf/Hair/MI_GingerHair.MI_GingerHair" :!type "MaterialInterface Object Reference"))
  (`PrimitiveComponent.SetMaterial` (`self.Hand1`) 0 (select `/Game/Data/EHair` (`self.Hair`) :`NewEnumerator0` "/Game/Dwarf/Hair/MI_BlondHair.MI_BlondHair" :`NewEnumerator1` "/Game/Dwarf/Hair/MI_GreyHair.MI_GreyHair" :`NewEnumerator2` "/Game/Dwarf/Hair/MI_GingerHair.MI_GingerHair" :!type "MaterialInterface Object Reference"))
  (`PrimitiveComponent.SetMaterial` (`self.Hand`) 0 (select `/Game/Data/EHair` (`self.Hair`) :`NewEnumerator0` "/Game/Dwarf/Hair/MI_BlondHair.MI_BlondHair" :`NewEnumerator1` "/Game/Dwarf/Hair/MI_GreyHair.MI_GreyHair" :`NewEnumerator2` "/Game/Dwarf/Hair/MI_GingerHair.MI_GingerHair" :!type "MaterialInterface Object Reference"))
  (`PrimitiveComponent.SetMaterial` (`self.Head`) 0 (select `/Game/Data/EHair` (`self.Hair`) :`NewEnumerator0` "/Game/Dwarf/Hair/MI_BlondHair.MI_BlondHair" :`NewEnumerator1` "/Game/Dwarf/Hair/MI_GreyHair.MI_GreyHair" :`NewEnumerator2` "/Game/Dwarf/Hair/MI_GingerHair.MI_GingerHair" :!type "MaterialInterface Object Reference"))
  (`PrimitiveComponent.SetMaterial` (`self.Body1`) 0 (select `/Game/Data/EClothes` (`self.Clothes`) :`NewEnumerator0` "/Game/Dwarf/Clothes/MI_RichClothes.MI_RichClothes" :`NewEnumerator1` "/Game/Dwarf/Clothes/MI_BrownClothes.MI_BrownClothes" :`NewEnumerator2` "/Game/Dwarf/Clothes/MI_IceClothes.MI_IceClothes" :!type "MaterialInterface Object Reference"))
  (`PrimitiveComponent.SetMaterial` (`self.LeftFoot1`) 0 (select `/Game/Data/EClothes` (`self.Clothes`) :`NewEnumerator0` "/Game/Dwarf/Clothes/MI_RichClothes.MI_RichClothes" :`NewEnumerator1` "/Game/Dwarf/Clothes/MI_BrownClothes.MI_BrownClothes" :`NewEnumerator2` "/Game/Dwarf/Clothes/MI_IceClothes.MI_IceClothes" :!type "MaterialInterface Object Reference"))
  (`PrimitiveComponent.SetMaterial` (`self.RightFoot1`) 0 (select `/Game/Data/EClothes` (`self.Clothes`) :`NewEnumerator0` "/Game/Dwarf/Clothes/MI_RichClothes.MI_RichClothes" :`NewEnumerator1` "/Game/Dwarf/Clothes/MI_BrownClothes.MI_BrownClothes" :`NewEnumerator2` "/Game/Dwarf/Clothes/MI_IceClothes.MI_IceClothes" :!type "MaterialInterface Object Reference"))
  (`PrimitiveComponent.SetMaterial` (`self.Body`) 0 (select `/Game/Data/EClothes` (`self.Clothes`) :`NewEnumerator0` "/Game/Dwarf/Clothes/MI_RichClothes.MI_RichClothes" :`NewEnumerator1` "/Game/Dwarf/Clothes/MI_BrownClothes.MI_BrownClothes" :`NewEnumerator2` "/Game/Dwarf/Clothes/MI_IceClothes.MI_IceClothes" :!type "MaterialInterface Object Reference"))
  (`PrimitiveComponent.SetMaterial` (`self.LeftFoot`) 0 (select `/Game/Data/EClothes` (`self.Clothes`) :`NewEnumerator0` "/Game/Dwarf/Clothes/MI_RichClothes.MI_RichClothes" :`NewEnumerator1` "/Game/Dwarf/Clothes/MI_BrownClothes.MI_BrownClothes" :`NewEnumerator2` "/Game/Dwarf/Clothes/MI_IceClothes.MI_IceClothes" :!type "MaterialInterface Object Reference"))
  (`PrimitiveComponent.SetMaterial` (`self.RightFoot`) 0 (select `/Game/Data/EClothes` (`self.Clothes`) :`NewEnumerator0` "/Game/Dwarf/Clothes/MI_RichClothes.MI_RichClothes" :`NewEnumerator1` "/Game/Dwarf/Clothes/MI_BrownClothes.MI_BrownClothes" :`NewEnumerator2` "/Game/Dwarf/Clothes/MI_IceClothes.MI_IceClothes" :!type "MaterialInterface Object Reference"))
  (`StaticMeshComponent.SetStaticMesh` (`self.WeaponMesh`) _returnvalue)
  (`StaticMeshComponent.SetStaticMesh` _weaponmesh1 _returnvalue)
  (`SceneComponent.SetRelativeScale3D` _weaponmesh1 (select `/Game/Data/EWeapon` _weapon :`NewEnumerator0` (7.5 7.5 7.5) :`NewEnumerator1` (15.0 15.0 15.0) :`NewEnumerator2` (10.0 10.0 10.0) :!type "Vector Structure"))
  (`SceneComponent.SetRelativeScale3D` (`self.WeaponMesh`) (select `/Game/Data/EWeapon` _weapon :`NewEnumerator0` (7.5 7.5 7.5) :`NewEnumerator1` (15.0 15.0 15.0) :`NewEnumerator2` (10.0 10.0 10.0) :!type "Vector Structure"))
  (bind _outrownames (`DataTableFunctionLibrary.GetDataTableRowNames` "/Game/Data/Names.Names"))
  (bind _returnvalue_2 (`|GetDataTableRow` "/Game/Data/Names.Names" (`KismetArrayLibrary.Array_Random` _outrownames))
    (:`then`
      (set `self.Name` (break `/Game/Data/SName` _returnvalue_2)))))

(fn `UserConstructionScript`
  (`parent.UserConstructionScript`))